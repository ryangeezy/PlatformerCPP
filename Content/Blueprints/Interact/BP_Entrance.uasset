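; BP_Entrance is an interactable entrance actor whose interaction volume is sized to its door.
; The construction script caches DoorExtent and passes it to SetDoorExtent, which scales the InteractVolume box's X extent while preserving Y and Z.
; When RequireVisibility is set, construction also resets Direction to zero.
; Overlap handling only forwards to the parent class, so the entrance's runtime behavior is not defined here.
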(event Collision|EventActorBeginOverlap
  (params (OtherActor :type Actor%20Object%20Reference))
  (|CallParentFunction OtherActor))

(fn ConstructionScript
  (bind _doorextent (Variables|DesignerEntrance|GetDoorExtent))
  (|CallParentFunction)
  (Variables|DesignerEntrance|SetCachedDoorExtent _doorextent)
  (CallFunction|SetDoorExtent _doorextent)
  (if (Variables|DesignerEntrance|GetRequireVisibility)
    (Variables|DesignerEntrance|SetDirection 0)))

(fn SetDoorExtent
  (params (DoorExtent :type Float%20%28single-precision%29))
  (bind _interactvolume (Variables|Default|GetInteractVolume))
  (bind _boxextent (Variables|/Script/Engine.BoxComponent|GetBoxExtent _interactvolume))
  (Components|Box|SetBoxExtent _interactvolume (Math|Vector|MakeVector (* DoorExtent 5e+01) (.y _boxextent) (.z _boxextent)) true))