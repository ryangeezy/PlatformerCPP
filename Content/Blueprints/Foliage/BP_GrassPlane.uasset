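; BP_GrassPlane is a foliage Blueprint that scatters grass static mesh components over a rectangular area.
; The Construction Script adds GrassAmount components at random X/Y positions between MinLoc and MaxLoc, all at a fixed vertical offset.
; Each gets random yaw and a random vertical stretch multiplied by Height.
; Placement uses unseeded randomness and individual components rather than instancing, and the event graph is empty.
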(event EventBeginPlay)

(event Collision|EventActorBeginOverlap
  (params (OtherActor :type Actor%20Object%20Reference)))

(event EventTick
  (params (DeltaSeconds :type Float%20%28single-precision%29)))

(fn ConstructionScript
  (bind _minloc (Variables|Default|GetminLoc))
  (bind _maxloc (Variables|Default|GetmaxLoc))
  (for _index (range 1 (Variables|Default|GetGrassAmount))
    (AddComponent|AddStaticMeshComponent false (Math|Transform|MakeTransform (Math|Vector|MakeVector (Math|Random|RandomFloatinRange (.x _minloc) (.x _maxloc)) (Math|Random|RandomFloatinRange (.y _minloc) (.y _maxloc)) -55.0) (Math|Rotator|MakeRotator 0.0 0.0 (Math|Random|RandomFloatinRange 0.0 3.6e+02)) (Math|Vector|MakeVector 1.0 1.0 (* (Math|Random|RandomFloatinRange 1.0 4.0) (Variables|Default|GetHeight)))))))