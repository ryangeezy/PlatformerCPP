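; BP_Entrance is an interactable platform entrance with a resizable interaction volume.
; Its construction script caches DoorExtent, then scales it to set the InteractVolume box's X extent, keeping Y and Z unchanged.
; Actor overlap handling is left to the parent class, as the event only forwards to it.
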(event Collision|EventActorBeginOverlap
  (params (OtherActor :type Actor%20Object%20Reference))
  (|CallParentFunction OtherActor))

(fn ConstructionScript
  (bind _doorextent (Variables|Designer_Entrance|GetDoorExtent))
  (|CallParentFunction)
  (Variables|Designer_Entrance|SetCachedDoorExtent _doorextent)
  (CallFunction|SetDoorExtent _doorextent))

(fn SetDoorExtent
  (params (DoorExtent :type Float%20%28single-precision%29))
  (bind _interactvolume (Variables|Default|GetInteractVolume))
  (bind _boxextent (Variables|/Script/Engine.BoxComponent|GetBoxExtent _interactvolume))
  (Components|Box|SetBoxExtent _interactvolume (Math|Vector|MakeVector (* DoorExtent 5e+01) (.y _boxextent) (.z _boxextent)) true))