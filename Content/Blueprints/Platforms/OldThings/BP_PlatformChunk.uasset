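; BP_PlatformChunk is a platform builder that fills a box-shaped volume with a grid of platform child actors.
; Its construction script loops over X, Y and Z between MinLoc and MaxLoc in 100-unit steps, adding a child actor component at each cell.
; Each child uses the Platform class if it casts to BP_PlatformStaticMaster, otherwise Platform falls back to BP_PlatformStaticBase.
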(fn ConstructionScript
  (bind _minloc (Variables|Default|GetminLoc))
  (bind _maxloc (Variables|Default|GetmaxLoc))
  (bind _returnvalue (- (.y _minloc) (.y _maxloc)))
  (bind _returnvalue_2 (- (.z _minloc) (.z _maxloc)))
  (bind _returnvalue_3 (- (.x _minloc) (.x _maxloc)))
  (bind _returnvalue_4 (/ _returnvalue 1e+02))
  (bind _returnvalue_5 (/ _returnvalue_2 1e+02))
  (bind _returnvalue_6 (/ _returnvalue_3 1e+02))
  (for _index (range 0 (Math|Integer|Absolute(Integer) (Math|Float|Truncate _returnvalue_6)))
    (for _index_2 (range 0 (Math|Integer|Absolute(Integer) (Math|Float|Truncate _returnvalue_4)))
      (for _index_3 (range 0 (Math|Integer|Absolute(Integer) (Math|Float|Truncate _returnvalue_5)))
        (bind _returnvalue_7 (AddComponent|AddChildActorComponent false (Math|Transform|MakeTransform (Math|Vector|MakeVector (* (* _index -1e+02) (Math|Float|Sign(Float) _returnvalue_6)) (* (* _index_2 -1e+02) (Math|Float|Sign(Float) _returnvalue_4)) (* (* _index_3 -1e+02) (Math|Float|Sign(Float) _returnvalue_5))) "0, 0, 0" "1,1,1")))
        (bind _asbp_platform_static_master (Utilities|Casting|CastToBP_PlatformStaticMasterClass (Variables|Default|GetPlatform))
          (:then
            (ChildActorComponent|SetChildActorClass _returnvalue_7 _asbp_platform_static_master))
          (:CastFailed
            (ChildActorComponent|SetChildActorClass _returnvalue_7 "/Game/Blueprints/Platforms/Master/BP_PlatformStaticBase.BP_PlatformStaticBase_C")
            (Variables|Default|SetPlatform "/Game/Blueprints/Platforms/Master/BP_PlatformStaticBase.BP_PlatformStaticBase_C")))))))