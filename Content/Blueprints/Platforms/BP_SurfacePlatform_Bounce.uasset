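; Bounce variant of a surface platform for the Dimense character, with the bounce itself currently disconnected.
; On a Top hit, it checks that the character is grounded and its feet lie within the inset bounds along the camera-right axis, but takes no action.
; Impulse and angled-velocity nodes targeting the old Fez character never run.
; Construction clamps the inset threshold to just under the shorter horizontal half-extent.
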(event OnComponentHit(Top)
  (params (HitComponent :type Primitive%20Component%20Object%20Reference) (OtherActor :type Actor%20Object%20Reference) (OtherComp :type Primitive%20Component%20Object%20Reference) (NormalImpulse :type Vector :default "0, 0, 0") (Hit :type Hit%20Result%20Structure%20%28by%20ref%29))
  (bind _top (Variables|Default|GetTop))
  (bind (_origin _boxextent) (Collision|GetComponentBounds _top))
  (bind _asbp_dimense_character (Utilities|Casting|CastToBP_DimenseCharacter OtherActor))
  (if (not (AI|Components|NavMovement|IsFalling (Variables|/Script/Engine.Character|GetCharacterMovement _asbp_dimense_character)))
    (if (Math|Float|NearlyEqual(Float) (Math|Float|Absolute(Float) (.x (Variables|/Script/PlatformerCPP.DimenseCharacter|GetCamRightVector _asbp_dimense_character))) 1.0 0.01)
      (if (< (Math|Float|Absolute(Float) (.x (- _origin (Math|Vector|MakeVector (.x (Variables|/Script/PlatformerCPP.DimenseCharacter|GetFootLocation _asbp_dimense_character)) (.y (Variables|/Script/PlatformerCPP.DimenseCharacter|GetFootLocation _asbp_dimense_character)) 0.0)))) (- (.x _boxextent) (Variables|Default|GetDistanceThreshold)))
        _)
      (elif (Math|Float|NearlyEqual(Float) (Math|Float|Absolute(Float) (.y (Variables|/Script/PlatformerCPP.DimenseCharacter|GetCamRightVector _asbp_dimense_character))) 1.0 0.01)
        (if (< (Math|Float|Absolute(Float) (.y (- _origin (Math|Vector|MakeVector (.x (Variables|/Script/PlatformerCPP.DimenseCharacter|GetFootLocation _asbp_dimense_character)) (.y (Variables|/Script/PlatformerCPP.DimenseCharacter|GetFootLocation _asbp_dimense_character)) 0.0)))) (- (.y _boxextent) (Variables|Default|GetDistanceThreshold)))
          _)))))

(fn ConstructionScript
  (bind _top (Variables|Default|GetTop))
  (bind _boxextent (Collision|GetComponentBounds _top))
  (|CallParentFunction)
  (if (>= (.x _boxextent) (.y _boxextent))
    (Variables|Default|SetDistanceThreshold (Math|Float|Clamp(Float) (Variables|Default|GetDistanceThreshold) 0.0 (- (.y _boxextent) 5.0)))
    (else
      (Variables|Default|SetDistanceThreshold (Math|Float|Clamp(Float) (Variables|Default|GetDistanceThreshold) 0.0 (- (.x _boxextent) 5.0))))))