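; Base platform actor that builds itself in the construction script from X/Y scale and height settings.
; It scales and materials a top Cube, adds an offset Bottom mesh when height exceeds one, and adds a surface component for surface platforms.
; Optional foliage scatters randomized instanced meshes over the top, though CreateFoliage is passed Grass yet loops on the flower total.
; Separate grass and flower functions are never called here, and BeginPlay is empty.
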(event EventBeginPlay
  ;[1 0.2109 0] Update Actor to reflect scale in Editor
)

(fn ConstructionScript
  (bind _cube (Variables|Default|GetCube))
  (bind _platformscalex (Variables|DesignerPlatform|GetPlatformScaleX))
  (bind _platformscaley (Variables|DesignerPlatform|GetPlatformScaleY))
  (bind _bottomscalez (Variables|DesignerPlatform|GetBottomScaleZ))
  (bind _returnvalue (* _platformscalex _platformscaley))
  (if (Variables|Default|GetbIsSurface)
    (AddComponent|AddSurfacePlatformComponent)
    (else
      (Variables|DesignerPlatform|SetSpawnFoliage false)))
  (Variables|Default|SetGrassFoliageTotal (* _returnvalue (Variables|DesignerPlatform|GetGrassFoliageCount)))
  (Variables|Default|SetFlowerFoliageTotal (* _returnvalue (Variables|DesignerPlatform|GetFlowerFoliageCount)))
  (Utilities|FlowControl|Sequence
    (:then_0
      (Rendering|Material|SetMaterial _cube 0 (Variables|DesignerPlatform|GetSurfaceMaterial))
      ;[0 1 0.03906] Setup Top
      (Transformation|SetRelativeTransform _cube (Math|Transform|MakeTransform "0, 0, 0" "0, 0, 0" (Math|Vector|MakeVector (Math|Conversions|ToFloat(Integer) (Variables|DesignerPlatform|GetPlatformScaleX)) (Math|Conversions|ToFloat(Integer) (Variables|DesignerPlatform|GetPlatformScaleY)) 1.0)) false false)
      ;[1 0.3984 0] If Height > 1
      (if (> _bottomscalez 1.0)
        ;[1 0.09375 0] Setup Bottom (Scale and Location are seperate so that the bounds calculation can happen after scaling)
        (bind _returnvalue_2 (AddComponent|AddStaticMeshComponent false))
        (bind _output_get (Variables|Default|SetBottom _returnvalue_2))
        (Transformation|SetRelativeScale3D _output_get (Math|Vector|MakeVector (Math|Conversions|ToFloat(Integer) (Variables|DesignerPlatform|GetPlatformScaleX)) (Math|Conversions|ToFloat(Integer) (Variables|DesignerPlatform|GetPlatformScaleY)) (- (Variables|DesignerPlatform|GetBottomScaleZ) 1.0)))
        (Transformation|SetRelativeLocation _output_get (Math|Vector|MakeVector 0.0 0.0 (- (* (.z (.BoxExtent (Collision|GetComponentBounds _output_get))) -1.0) (.z (.BoxExtent (Collision|GetComponentBounds _cube))))) false false)
        (Rendering|Material|SetMaterial _output_get 0 (Variables|DesignerPlatform|GetBelowSurfaceMaterial))
        (else
          (Transformation|SetRelativeScale3D (Variables|Default|GetCube) (Math|Vector|MakeVector (Math|Conversions|ToFloat(Integer) (Variables|DesignerPlatform|GetPlatformScaleX)) (Math|Conversions|ToFloat(Integer) (Variables|DesignerPlatform|GetPlatformScaleY)) _bottomscalez)))))
    (:then_1
      (if (Variables|DesignerPlatform|GetSpawnFoliage)
        ;[0 0.3437 1] Spawn Foliage
        (CallFunction|CreateFoliage (Variables|Default|GetGrass))))))

(fn CreateFoliage
  (params (StaticMesh :type Static%20Mesh%20Object%20Reference))
  (bind _foliageradius (Variables|DesignerPlatform|GetFoliageRadius))
  (bind _foliagepadding (Variables|DesignerPlatform|GetFoliagePadding))
  (bind _foliageseperation (Variables|DesignerPlatform|GetFoliageSeperation))
  (bind _returnvalue (AddComponent|AddInstancedStaticMeshComponent true))
  (Components|StaticMesh|SetStaticMesh _returnvalue StaticMesh)
  (Transformation|AttachComponentToComponent _returnvalue 0 "None" (Variables|Default|GetAttachToComponentLocationRule) "KeepWorld" "KeepWorld" false)
  (for _index (range 1 (Variables|Default|GetFlowerFoliageTotal))
    (Components|InstancedStaticMesh|AddInstance _returnvalue (Math|Transform|MakeTransform (+ (Transformation|GetWorldLocation (Variables|Default|GetCube)) (+ (Math|Vector|MakeVector (|((((Scale-Padding)*0.500000)*Speration)*Random) (Math|Conversions|ToFloat(Integer) (Variables|DesignerPlatform|GetPlatformScaleX)) _foliageseperation (Math|Random|RandomFloatinRange -1.0 1.0) _foliagepadding) (|((((Scale-Padding)*0.500000)*Speration)*Random) (Math|Conversions|ToFloat(Integer) (Variables|DesignerPlatform|GetPlatformScaleY)) _foliageseperation (Math|Random|RandomFloatinRange -1.0 1.0) _foliagepadding) 0.0) "0, 0,50.000000")) (Math|Rotator|MakeRotator 0.0 0.0 (Math|Random|RandomFloatinRange 0.0 3.6e+02)) (Math|Vector|MakeVector _foliageradius _foliageradius (Math|Random|RandomFloatinRange (Variables|DesignerPlatform|GetFoliageMinHeight) (Variables|DesignerPlatform|GetFoliageMaxHeight))))))
  (return))

(fn AddInstancedFlowers
  (bind _foliageradius (Variables|DesignerPlatform|GetFoliageRadius))
  (bind _foliagepadding (Variables|DesignerPlatform|GetFoliagePadding))
  (bind _foliageseperation (Variables|DesignerPlatform|GetFoliageSeperation))
  (bind _flowerheight (Variables|DesignerPlatform|GetFlowerHeight))
  (bind _returnvalue (AddComponent|AddInstancedStaticMeshComponent true))
  (Components|StaticMesh|SetStaticMesh _returnvalue 0)
  (Transformation|AttachComponentToComponent _returnvalue 0 "None" (Variables|Default|GetAttachToComponentLocationRule) "KeepWorld" "KeepWorld" false)
  (for _index (range 1 (Variables|Default|GetFlowerFoliageTotal))
    (Components|InstancedStaticMesh|AddInstance _returnvalue (Math|Transform|MakeTransform (+ (Transformation|GetWorldLocation (Variables|Default|GetCube)) (+ (Math|Vector|MakeVector (|((((Scale-Padding)*0.500000)*Speration)*Random) (Math|Conversions|ToFloat(Integer) (Variables|DesignerPlatform|GetPlatformScaleX)) _foliageseperation (Math|Random|RandomFloatinRange -1.0 1.0) _foliagepadding) (|((((Scale-Padding)*0.500000)*Speration)*Random) (Math|Conversions|ToFloat(Integer) (Variables|DesignerPlatform|GetPlatformScaleY)) _foliageseperation (Math|Random|RandomFloatinRange -1.0 1.0) _foliagepadding) (* (Variables|Default|GetSurfaceOffset) -1.0)) "0, 0,50.000000")) (Math|Rotator|MakeRotator 0.0 0.0 (Math|Random|RandomFloatinRange 0.0 3.6e+02)) (Math|Vector|MakeVector _foliageradius _foliageradius (Math|Random|RandomFloatinRange _flowerheight (+ _flowerheight (Variables|DesignerPlatform|GetFlowerHeightVariation)))))))
  (return))

(fn AddInstancedGrass
  (bind _foliageradius (Variables|DesignerPlatform|GetFoliageRadius))
  (bind _foliagepadding (Variables|DesignerPlatform|GetFoliagePadding))
  (bind _foliageseperation (Variables|DesignerPlatform|GetFoliageSeperation))
  (bind _grassheight (Variables|DesignerPlatform|GetGrassHeight))
  (bind _returnvalue (AddComponent|AddInstancedStaticMeshComponent true))
  (Components|StaticMesh|SetStaticMesh _returnvalue 0)
  (Transformation|AttachComponentToComponent _returnvalue 0 "None" (Variables|Default|GetAttachToComponentLocationRule) "KeepWorld" "KeepWorld" false)
  (for _index (range 1 (Variables|Default|GetGrassFoliageTotal))
    (Components|InstancedStaticMesh|AddInstance _returnvalue (Math|Transform|MakeTransform (+ (Transformation|GetWorldLocation (Variables|Default|GetCube)) (+ (Math|Vector|MakeVector (|((((Scale-Padding)*0.500000)*Speration)*Random) (Math|Conversions|ToFloat(Integer) (Variables|DesignerPlatform|GetPlatformScaleX)) _foliageseperation (Math|Random|RandomFloatinRange -1.0 1.0) _foliagepadding) (|((((Scale-Padding)*0.500000)*Speration)*Random) (Math|Conversions|ToFloat(Integer) (Variables|DesignerPlatform|GetPlatformScaleY)) _foliageseperation (Math|Random|RandomFloatinRange -1.0 1.0) _foliagepadding) (* (Variables|Default|GetSurfaceOffset) -1.0)) "0, 0,50.000000")) (Math|Rotator|MakeRotator 0.0 0.0 (Math|Random|RandomFloatinRange 0.0 3.6e+02)) (Math|Vector|MakeVector _foliageradius _foliageradius (Math|Random|RandomFloatinRange _grassheight (+ _grassheight (Variables|DesignerPlatform|GetGrassHeightVariation)))))))
  (return))