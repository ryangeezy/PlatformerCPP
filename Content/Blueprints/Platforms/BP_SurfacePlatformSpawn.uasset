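; BP_SurfacePlatformSpawn is a platform actor built from a Top and a Bottom component, with separate surface and below-surface materials set in the construction script.
; UpdatePlatform applies X and Y scale to the actor, keeping its Z scale at one.
; When requested height exceeds one, Bottom takes the extra height and is positioned beneath Top using component bounds.
; Otherwise it hides Bottom, leaving only the surface layer.
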(event Custom|UpdatePlatform
  (params (Scale :type Vector))
  (bind _top (Variables|Default|GetTop))
  (bind _bottom (Variables|Default|GetBottom))
  (bind _output_get (Variables|Default|SetPlatformScale (Math|Vector|MakeVector (.x Scale) (.y Scale) (.z Scale))))
  (Transformation|SetActorScale3D (Math|Vector|MakeVector (.x _output_get) (.y _output_get) 1.0))
  (if (> (.z _output_get) 1.0)
    (Transformation|SetRelativeTransform _top (Math|Transform|MakeTransform "0, 0, 0" "0, 0, 0" "1,1,1") false false)
    (Transformation|SetRelativeScale3D _bottom (Math|Vector|MakeVector 1.0 1.0 (- (.z _output_get) 1.0)))
    (Transformation|SetRelativeLocation (Variables|Default|GetBottom) (Math|Vector|MakeVector 0.0 0.0 (- (* (.z (.BoxExtent (Collision|GetComponentBounds _bottom))) -1.0) (.z (.BoxExtent (Collision|GetComponentBounds _top))))) false false)
    (else
      (Rendering|SetVisibility (Variables|Default|GetBottom) false false))))

(fn ConstructionScript
  (Rendering|Material|SetMaterial (Variables|Default|GetTop) 0 (Variables|Default|GetSurfaceMaterial))
  (Rendering|Material|SetMaterial (Variables|Default|GetBottom) 0 (Variables|Default|GetBelowSurfaceMaterial)))