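; Work-in-progress platform selector actor that shows a chosen platform class as a child actor.
; The construction script adds a child actor component, stores it as PlatformObject and sets it to PlatformClass.
; PreviousPlatform finds the current class in PlatformClasses and swaps the child to the preceding entry, clamping at the first instead of wrapping.
; NextPlatform is still an empty stub, and the event graph has no active logic.
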(event EventBeginPlay)

(event Collision|EventActorBeginOverlap
  (params (OtherActor :type Actor%20Object%20Reference)))

(event EventTick
  (params (DeltaSeconds :type Float%20%28single-precision%29)))

(fn ConstructionScript
  (bind _returnvalue (AddComponent|AddChildActorComponent false))
  (Variables|Default|SetPlatformObject _returnvalue)
  (ChildActorComponent|SetChildActorClass _returnvalue (Variables|Default|GetPlatformClass)))

(fn PreviousPlatform
  (bind _platformclasses (Variables|Default|GetPlatformClasses))
  ;[1 1 1] WIP
  (bind (_array_element _array_index) (Utilities|Array|ForEachLoopwithBreak _platformclasses :!label _label)
    (:LoopBody
      (if (== (Variables|Default|GetPlatformClass) _array_element)
        (bind _output_get (Variables|Default|SetPlatformClass (Utilities|Array|Get(acopy) _platformclasses (Math|Integer|Clamp(Integer) (- _array_index 1) 0 (Utilities|Array|LastIndex _platformclasses)))))
        (ChildActorComponent|SetChildActorClass (Variables|Default|GetPlatformObject) _output_get)
        (goto _label Break)))))

(fn NextPlatform
  ;[1 1 1] WIP
)