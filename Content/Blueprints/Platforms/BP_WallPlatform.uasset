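; BP_WallPlatform is a platform actor that builds itself in the construction script from a Scale variable snapped to whole numbers.
; The actor scales only in X and Y, keeping the Top mesh one unit tall with SurfaceMaterial.
; When Z exceeds one, it adds a Bottom mesh for the remaining height, offset beneath Top using component bounds and given UnderMaterial.
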(fn ConstructionScript
  (bind _top (Variables|Default|GetTop))
  (Rendering|Material|SetMaterial (Variables|Default|GetTop) 0 (Variables|Default|GetSurfaceMaterial))
  (bind _output_get (Variables|Default|SetScale (Math|Vector|MakeVector (Math|Conversions|ToFloat(Integer) (Math|Float|Round (.x (Variables|Default|GetScale)))) (Math|Conversions|ToFloat(Integer) (Math|Float|Round (.y (Variables|Default|GetScale)))) (Math|Conversions|ToFloat(Integer) (Math|Float|Round (.z (Variables|Default|GetScale)))))))
  (Transformation|SetActorScale3D (Math|Vector|MakeVector (.x _output_get) (.y _output_get) 1.0))
  (if (> (.z _output_get) 1.0)
    (bind _returnvalue (AddComponent|AddStaticMeshComponent false))
    (Variables|Default|SetBottom _returnvalue)
    (Transformation|SetRelativeTransform _top (Math|Transform|MakeTransform "0, 0, 0" "0, 0, 0" "1,1,1") false false)
    (Transformation|SetRelativeScale3D (Variables|Default|GetBottom) (Math|Vector|MakeVector 1.0 1.0 (- (.z _output_get) 1.0)))
    (Transformation|SetRelativeLocation (Variables|Default|GetBottom) (Math|Vector|MakeVector 0.0 0.0 (- (* (.z (.BoxExtent (Collision|GetComponentBounds (Variables|Default|GetBottom)))) -1.0) (.z (.BoxExtent (Collision|GetComponentBounds _top))))) false false)
    (Rendering|Material|SetMaterial (Variables|Default|GetBottom) 0 (Variables|Default|GetUnderMaterial))))