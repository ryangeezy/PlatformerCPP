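; Player character Blueprint for a camera-rotating platformer, wiring movement, jump and drop-down, camera rotation, fall-death respawn, and door level loading gated by camera side.
; Tick checks fall death and box-traces from main to opposite camera, collecting depth-spanning pickups that can trace back to the player.
; BeginPlay creates debug/config widgets whose values retune movement and cameras.
; Debug keys drive a separate capture camera; the older ground/head trace logic is disconnected.
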(event EventTick
  (params (DeltaSeconds :type Float%20%28single-precision%29))
  ;[0.4155 0.4155 0.4155] Tick
  (Utilities|FlowControl|Sequence
    (:then_0
      (if (Class|DimenseCharacter|IsFallingDownward)
        (bind _returnvalue (Class|DimenseCharacter|CheckDeathbyFallDistance))
        (Utilities|Respawn _returnvalue)))
    (:then_1
      ;;[0.1028 1 0] Check for pickups
      (Pickups|BoxTraceforMultiPickupObjects))))

(event EventResetCanMoveAround
  ;[0.3974 0 1] Timers
  (Variables|Default|SetbCanMoveAround true))

(event EventResetCanTransport
  ;[0.3974 0 1] Timers
  (Variables|Default|SetbCanTransport true))

(event EventBeginPlay
  (bind _charactermovement (Variables|Character|GetCharacterMovement))
  (bind _cameraprezoomstartx (Variables|Camera|GetCameraPreZoomStartX))
  (bind _maincamera (Variables|Default|GetMainCamera))
  ;[1 0.02563 0] Begin Play
  (bind _returnvalue (Settings|GetGameUserSettings))
  (Class|GameUserSettings|SetVSyncEnabled _returnvalue true)
  (Variables|Movement|SetStartLocation (Variables|/Script/Engine.SceneComponent|GetRelativeLocation (Variables|Default|GetPhysicsComp)))
  (Utilities|Array|Add (Variables|Default|GetPickupIgnoreActors) self)
  (bind _asbp_player_controller (Utilities|Casting|CastToBP_PlayerController (Game|GetPlayerController 0)))
  (bind _output_get (Variables|Movement|SetPlayerController _asbp_player_controller))
  (bind _returnvalue_2 (UserInterface|CreateWidget "/Game/Blueprints/System/BPW_PnP.BPW_PnP_C" _output_get))
  (bind _returnvalue_3 (UserInterface|CreateWidget "/Game/Blueprints/System/BPW_PlayerConfig.BPW_PlayerConfig_C" _output_get))
  (UserInterface|Viewport|AddtoViewport _returnvalue_2 0)
  ;;[0.4688 0.7379 1] Config
  (Default|BPIPlayerSetConfig _returnvalue_3 (Utilities|Struct|MakeSTR_PlayerConfig (Variables|/Script/Engine.CharacterMovementComponent|GetMaxWalkSpeed _charactermovement) (Variables|Default|GetWalkAcceleration) (Variables|/Script/Engine.CharacterMovementComponent|GetGroundFriction _charactermovement) (Variables|Default|GetMeshRotationTime) (Variables|/Script/Engine.CharacterMovementComponent|GetAirControl _charactermovement) (Variables|Default|GetGroundTraceLength) (Variables|/Script/Engine.SpringArmComponent|GetTargetArmLength (Variables|Default|GetMainCameraSpringArm)) 0.0 (Variables|/Script/Engine.CharacterMovementComponent|GetJumpZVelocity _charactermovement) (Variables|Default|GetbDebug)))
  (if (Variables|Camera|GetbDoZoom)
    (Transformation|AddLocalOffset _maincamera (Math|Vector|MakeVector _cameraprezoomstartx 0.0 0.0) false false)
    (Utilities|FlowControl|Sequence
      (:then_1
        (bind _xlocation (Timeline|Timeline PlayFromStart)
          (:Update
            (Transformation|SetRelativeLocation _maincamera (Math|Vector|MakeVector (Math|Float|Lerp _cameraprezoomstartx 0.0 _xlocation) 0.0 0.0) false false)))))))

(event EventBPIConfigSetPlayer
  (params (PlayerConfig :type STR%20Player%20Config%20Structure))
  (bind _charactermovement (Variables|Character|GetCharacterMovement))
  ;[1 0.02563 0] Begin Play
  ;;[0.4688 0.7379 1] Config
  (Variables|/Script/Engine.CharacterMovementComponent|SetMaxWalkSpeed _charactermovement (.maxwalkvelocity PlayerConfig))
  (Variables|Default|SetWalkAcceleration (.walkacceleration PlayerConfig))
  (Variables|/Script/Engine.CharacterMovementComponent|SetGroundFriction _charactermovement (.friction PlayerConfig))
  (Variables|Default|SetMeshRotationTime (.playerrotatetime PlayerConfig))
  (Variables|/Script/Engine.CharacterMovementComponent|SetAirControl _charactermovement (.aircontrol PlayerConfig))
  (Variables|Default|SetGroundTraceLength (.recentgroundchecklength PlayerConfig))
  (bind _output_get (Variables|/Script/Engine.SpringArmComponent|SetTargetArmLength (Variables|Default|GetMainCameraSpringArm) (.cameraboomlength PlayerConfig)))
  (Variables|/Script/Engine.SpringArmComponent|SetTargetArmLength (Variables|Default|GetAntiCameraSpringArm) (* -1 _output_get))
  (Variables|/Script/Engine.CharacterMovementComponent|SetJumpZVelocity _charactermovement (.jumpvelocity PlayerConfig))
  (Variables|Default|SetbDebug (.bdebugplatforms PlayerConfig)))

(event EventStartCanMoveAroundTimer
  ;[0.3974 0 1] Timers
  (Variables|Default|SetbCanMoveAround false)
  (Utilities|Time|SetTimerbyEvent (delegate EventResetCanMoveAround) 0.2))

(event EventStartCanTransportTimer
  ;[0.3974 0 1] Timers
  (Variables|Default|SetbCanTransport false)
  (Utilities|Time|SetTimerbyEvent (delegate EventResetCanTransport) 0.2))

(event Input|ActionEvents|InputActionJump
  (params (Key :type Key%20Structure :default "None"))
  ;[0.3144 1 0] Input
  (:Pressed
    (Variables|Default|SetbJumpPressed true)
    (if (Variables|Default|GetbMoveDownPressed)
      (Class|DimenseCharacter|JumpDown)
      (else
        (Character|Jump))))
  (:Released
    (Variables|Default|SetbJumpPressed false)
    (Character|StopJumping)))

(event Input|ActionEvents|InputActionRotateLeft
  (params (Key :type Key%20Structure :default "None"))
  ;[0.3144 1 0] Input
  (:Pressed
    (Class|DimenseCharacter|RotateCamera (Variables|Camera|GetCameraRotationDegrees))))

(event Input|ActionEvents|InputActionRotateRight
  (params (Key :type Key%20Structure :default "None"))
  ;[0.3144 1 0] Input
  (:Pressed
    (Class|DimenseCharacter|RotateCamera (* (Variables|Camera|GetCameraRotationDegrees) -1.0))))

(event Input|ActionEvents|InputActionDeveloperReset
  (params (Key :type Key%20Structure :default "None"))
  ;[0.3144 1 0] Input
  ;;[1 0.4463 0] Dev Tools
  (:Pressed
    (Transformation|SetActorLocation (Variables|Default|GetGroundLocation) false false)))

(event Input|ActionEvents|InputActionPanDebug
  (params (Key :type Key%20Structure :default "None"))
  ;[1 0.4463 0] Debug Camera
  (:Pressed
    (Variables|Debug|SetbDebugPanActive true))
  (:Released
    (Variables|Debug|SetbDebugPanActive false)))

(event Input|AxisEvents|InputAxisMoveDown
  (params (AxisValue :type Float%20%28single-precision%29))
  ;[0.3144 1 0] Input
  (Variables|Default|SetbMoveDownPressed (< AxisValue (+ -1.0 (Variables|Movement|GetJumpDownDeadZone)))))

(event Input|AxisEvents|InputAxisMoveLeftRight
  (params (AxisValue :type Float%20%28single-precision%29))
  ;[0.3144 1 0] Input
  (Class|DimenseCharacter|MoveLeftRight AxisValue))

(event Input|AxisEvents|InputAxisClimb_Enter
  (params (AxisValue :type Float%20%28single-precision%29))
  ;[0 0.4821 1] Load level by door
  (Utilities|LoadLevelbyDoor AxisValue))

(event Input|MouseEvents|MouseWheelAxis
  (params (AxisValue :type Float%20%28single-precision%29))
  ;[1 0.4463 0] Debug Camera
  (Debug|DebugCameraZoom AxisValue))

(event Input|MouseEvents|MouseY
  (params (AxisValue :type Float%20%28single-precision%29))
  ;[1 0.4463 0] Debug Camera
  (Debug|DebugCameraFreeRotation AxisValue (stale Input|MouseEvents|MouseX AxisValue)))

(event Input|MouseEvents|MouseX
  (params (AxisValue :type Float%20%28single-precision%29))
  ;[1 0.4463 0] Debug Camera
  (Debug|DebugPan AxisValue (stale Input|MouseEvents|MouseY AxisValue)))

(event Input|MouseEvents|MouseY
  (params (AxisValue :type Float%20%28single-precision%29))
  ;[1 0.4463 0] Debug Camera
  (Debug|DebugPan (stale Input|MouseEvents|MouseX AxisValue) AxisValue))

(event Input|MouseEvents|MouseX
  (params (AxisValue :type Float%20%28single-precision%29))
  ;[1 0.4463 0] Debug Camera
  (Debug|DebugCameraFreeRotation (stale Input|MouseEvents|MouseY AxisValue) AxisValue))

(event Input|KeyboardEvents|F
  (params (Key :type Key%20Structure :default "None"))
  ;[1 0.4463 0] Debug Camera
  (:Pressed
    (Utilities|DebugCamera90Rotation)))

(event Input|KeyboardEvents|H
  (params (Key :type Key%20Structure :default "None"))
  ;[0.3144 1 0] Input
  ;;[1 0.4463 0] Debug Toggle Keys
  (:Pressed
    (Utilities|FlowControl|FlipFlop
      (:A
        (Widget|SetVisibility (stale EventBeginPlay _returnvalue_2) "Hidden"))
      (:B
        (Widget|SetVisibility (stale EventBeginPlay _returnvalue_2) "Visible")))))

(event Input|KeyboardEvents|J
  (params (Key :type Key%20Structure :default "None"))
  (bind _pnpcapture (Variables|Default|GetPnPCapture))
  ;[1 0.4463 0] Debug Camera
  (:Pressed
    (Utilities|FlowControl|FlipFlop
      (:A
        (Variables|/Script/Engine.SceneCaptureComponent2D|SetbEnableClipPlane _pnpcapture true))
      (:B
        (Variables|/Script/Engine.SceneCaptureComponent2D|SetbEnableClipPlane _pnpcapture false)))))

(event Input|KeyboardEvents|G
  (params (Key :type Key%20Structure :default "None"))
  ;[1 0.4463 0] Debug Camera
  (:Pressed
    (Debug|DebugChangeCameraAngle)))

(event Input|KeyboardEvents|P
  (params (Key :type Key%20Structure :default "None"))
  ;[0.3144 1 0] Input
  ;;[1 0.4463 0] Debug Toggle Keys
  (:Pressed
    (Utilities|FlowControl|FlipFlop
      (:A
        (Widget|SetVisibility (stale EventBeginPlay _returnvalue_3) "Hidden"))
      (:B
        (Widget|SetVisibility (stale EventBeginPlay _returnvalue_3) "Visible")))))

(event Input|MouseEvents|RightMouseButton
  (params (Key :type Key%20Structure :default "None"))
  ;[1 0.4463 0] Debug Camera
  (:Pressed
    (Utilities|DebugCameraRotationSwitch :!label _label))
  (:Released
    (goto _label Released)))

(fn ConstructionScript)

(fn BoxTraceforMultiPickupObjects
  (bind _mywidth (Variables|Default|GetMyWidth))
  (bind _returnvalue (* _mywidth 0.5))
  (if (not (Variables|Default|GetbSpinning))
    (bind _outhits (Class|KismetSystemLibrary|BoxTraceMultiforObjects (Transformation|GetWorldLocation (Variables|Default|GetMainCamera)) (Transformation|GetWorldLocation (Variables|Default|GetAntiCameraSceneComponent)) (Math|Vector|MakeVector _returnvalue _returnvalue (* (Variables|Default|GetMyHeight) 0.5)) "0, 0, 0" (Variables|Default|GetPickupObjectTypes) false (Variables|Default|GetPickupIgnoreActors) "None" true "(R=1.000000,G=0.000000,B=0.000000,A=1.000000)" "(R=0.000000,G=1.000000,B=0.000000,A=1.000000)" 0.25))
    (for _array_element _outhits
      (bind _aspickup (Utilities|Casting|CastToPickup (.HitActor (Collision|BreakHitResult _array_element))))
      (bind _returnvalue_2 (Class|Pickup|AttemptTraceBacktoPlayer _aspickup))
      (if _returnvalue_2
        (Actor|DestroyActor _aspickup)))))

(fn DebugChangeCameraAngle
  (bind _pnpcapturespringarm (Variables|Default|GetPnPCaptureSpringArm))
  (if (and (not (Variables|Debug|GetbDebugCameraIsFlipping)) (not (Variables|Debug|GetbDebugCameraIsRotating)))
    (if (Variables|Debug|GetbDebugCameraToggle)
      (Transformation|SetRelativeRotation _pnpcapturespringarm (Variables|Debug|GetDebugCameraLastRotation45) false false)
      (Variables|Debug|SetbDebugCameraToggle false)
      (else
        (Transformation|SetRelativeRotation _pnpcapturespringarm (Variables|Debug|GetDebugCameraLastRotation90) false false)
        (Variables|Debug|SetbDebugCameraToggle true)))))

(fn DebugCameraFreeRotation
  (params (X :type Float%20%28single-precision%29) (Y :type Float%20%28single-precision%29))
  (bind _debugcamerarotationspeed (Variables|Debug|GetDebugCameraRotationSpeed))
  (if (and (Variables|Debug|GetbDebugCameraIsRotating) (not (Variables|Debug|GetbDebugCameraIsFlipping)))
    (Transformation|AddRelativeRotation (Variables|Default|GetPnPCaptureSpringArm) (Math|Rotator|MakeRotator 0.0 (* X _debugcamerarotationspeed) (* Y _debugcamerarotationspeed)) false false)))

(fn DebugCameraZoom
  (params (Axis :type Float%20%28single-precision%29))
  (bind _pnpcapturespringarm (Variables|Default|GetPnPCaptureSpringArm))
  (Variables|/Script/Engine.SpringArmComponent|SetTargetArmLength _pnpcapturespringarm (+ (* (Variables|Debug|GetDebugCameraZoomSpeed) Axis) (Variables|/Script/Engine.SpringArmComponent|GetTargetArmLength _pnpcapturespringarm))))

(fn DebugPan
  (params (X :type Float%20%28single-precision%29) (Y :type Float%20%28single-precision%29))
  (bind _pnpcapture (Variables|Default|GetPnPCapture))
  (bind _debugcamerapanspeed (Variables|Debug|GetDebugCameraPanSpeed))
  (if (Variables|Debug|GetbDebugPanActive)
    (Transformation|AddLocalOffset _pnpcapture (+ (* (Math|Vector|GetRightVector _pnpcapture) (* X _debugcamerapanspeed)) (* (Math|Vector|GetUpVector _pnpcapture) (* Y _debugcamerapanspeed))) false false)))

(fn DebugSetClipPlane
  (bind _pnpcapture (Variables|Default|GetPnPCapture))
  (bind _output_get (Variables|/Script/Engine.SceneCaptureComponent2D|SetClipPlaneNormal _pnpcapture (Math|Vector|GetForwardVector _pnpcapture)))
  (Variables|/Script/Engine.SceneCaptureComponent2D|SetClipPlaneBase _pnpcapture (- (Transformation|GetWorldLocation (Variables|Default|GetCube)) (* _output_get (Variables|Debug|GetDebugCameraClipPlaneDistance)))))