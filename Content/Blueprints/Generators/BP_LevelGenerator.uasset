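; BP_LevelGenerator builds an endless procedural path by spawning random chunk actors on a looping timer, starting from a grass chunk.
; Each chunk is placed beside the previous one using both box component extents along the current direction, and rotated to match it.
; Occasional random turns pick one of six directions, excluding the current and its paired one.
; The oldest chunks are destroyed beyond a maximum count, and the gap logic is never executed.
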(event Custom|Spawn%20Platforms
  (bind _activechunks (Variables|Default|GetActiveChunks))
  (bind _chunks (Variables|Default|GetChunks))
  (bind _returnvalue (Game|SpawnActorfromClass (Utilities|Array|Get(acopy) _chunks (Math|Random|RandomIntegerinRange 0 (- (Utilities|Array|Length _chunks) 1))) (Math|Transform|MakeTransform (Transformation|GetWorldLocation (Variables|Default|GetDefaultSceneRoot)) "0, 0, 0" "1,1,1") "Undefined" 0 0))
  (bind _output_get (Variables|Default|SetThisChunk _returnvalue))
  (Utilities|Array|Add _activechunks _output_get)
  (bind (_location _rotation) (CallFunction|SetTransform))
  (Transformation|SetActorTransform (Variables|Default|GetThisChunk) (Math|Transform|MakeTransform _location _rotation "1,1,1"))
  (Variables|Default|SetLastChunk (Variables|Default|GetThisChunk))
  (CallFunction|RemoveOldestPlatform (Variables|Default|GetMaxNumPlatforms))
  (Development|PrintString (Utilities|String|ToString(Integer) (Utilities|Array|Length _activechunks))))

(event EventBeginPlay
  (bind _returnvalue (Game|SpawnActorfromClass "/Game/Blueprints/Platforms/Chunks/BP_ChunkGrass3x3x1_.BP_ChunkGrass3x3x1__C" (Math|Transform|MakeTransform (Transformation|GetWorldLocation (Variables|Default|GetDefaultSceneRoot)) "0, 0, 0" "1,1,1") "Undefined" 0 0))
  (bind _output_get (Variables|Default|SetLastChunk _returnvalue))
  (Utilities|Array|Add (Variables|Default|GetActiveChunks) _output_get)
  (Utilities|Time|SetTimerbyEvent (delegate Custom|Spawn%20Platforms) (Variables|Default|GetGenerationSpeed) true))

(fn ConstructionScript
  (|CallParentFunction))

(fn SetTransform
  (bind _currentdirection (Variables|Default|GetCurrentDirection))
  (bind _lastchunk (Variables|Default|GetLastChunk))
  (if (Variables|Default|GetPickNewDirection?)
    (CallFunction|NewDirection))
  (Variables|Default|SetLocation (+ (Transformation|GetActorLocation _lastchunk) (* (+ (.BoxExtent (Collision|GetComponentBounds (Actor|GetComponentbyClass _lastchunk "/Script/Engine.BoxComponent"))) (.BoxExtent (Collision|GetComponentBounds (Actor|GetComponentbyClass (Variables|Default|GetThisChunk) "/Script/Engine.BoxComponent")))) (Utilities|Array|Get(acopy) (Variables|Default|GetDirections) _currentdirection))))
  (if (or (== _currentdirection 0) (== _currentdirection 1))
    (Variables|Default|SetRotation "0, 0, 0")
    (else
      (Variables|Default|SetRotation "0.000000,90.000000,0.000000")))
  (Variables|Default|SetPickNewDirection? (> (Math|Random|RandomFloat) 0.85))
  (return (Variables|Default|GetLocation) (Variables|Default|GetRotation)))

(fn NewDirection
  (while (Math|Boolean|ORBoolean (== (Variables|Default|GetCurrentDirection) (Variables|Default|GetTriedDirection)) (and (== (Variables|Default|GetCurrentDirection) 1) (== (Variables|Default|GetTriedDirection) 0)) (and (== (Variables|Default|GetCurrentDirection) 0) (== (Variables|Default|GetTriedDirection) 1)) (and (== (Variables|Default|GetCurrentDirection) 3) (== (Variables|Default|GetTriedDirection) 2)) (and (== (Variables|Default|GetCurrentDirection) 2) (== (Variables|Default|GetTriedDirection) 3)) (and (== (Variables|Default|GetCurrentDirection) 5) (== (Variables|Default|GetTriedDirection) 4)) (and (== (Variables|Default|GetCurrentDirection) 4) (== (Variables|Default|GetTriedDirection) 5)))
    (Variables|Default|SetTriedDirection (Math|Random|RandomIntegerinRange 0 5)))
  (Variables|Default|SetCurrentDirection (Variables|Default|GetTriedDirection))
  (Variables|Default|SetPickNewDirection? false)
  (return))

(fn RemoveOldestPlatform
  (params (MaxNumPlatforms :type Integer))
  (bind _activechunks (Variables|Default|GetActiveChunks))
  (if (> (Utilities|Array|Length _activechunks) MaxNumPlatforms)
    (Actor|DestroyActor (Utilities|Array|Get(acopy) _activechunks))
    (Utilities|Array|RemoveIndex _activechunks)))